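; BPC_Buffs is a character component that stores a list of active buffs, such as resistances, speed and damage.
; AddBuff and RemoveBuff edit the array and fire BuffAdded and BuffRemoved dispatchers.
; GetTotalBuffValue sums every buff's value, ignoring its Type input because the type comparison is unconnected.
; Tick draws a row of debug spheres above the owner, colored by buff type.
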(event `self.ReceiveTick`
  (params (DeltaSeconds :type "Float (single-precision)"))
  (for (_array_element _array_index) (`self.Buffs`)
    (`KismetSystemLibrary.DrawDebugSphere` (+ (`Actor.K2_GetActorLocation` (`self.GetOwner`)) (0.0 0.0 150.0) (* _array_index (20.0 0.0 0.0))) 5.0 12 (select `/Game/Characters/Structs/ENUM_BuffType` (`.Type_3_542718354D732257E7F3FEB61A2928C5` (break `/Game/Characters/Structs/Struct_Buff` _array_element)) :`NewEnumerator0` (struct :`R` 0.34003 :`G` 0.34003 :`B` 0.34003 :`A` 1.0) :`NewEnumerator3` (struct :`R` 1.0 :`G` 0.800806 :`A` 1.0) :`NewEnumerator4` (struct :`R` 0.10327 :`G` 1.0 :`A` 1.0) :`NewEnumerator5` (struct :`R` 0.080188 :`B` 1.0 :`A` 1.0) :`NewEnumerator6` (struct :`R` 1.0 :`G` 0.029312 :`B` 0.023066 :`A` 1.0) :`NewEnumerator2` (struct :`R` 0.126164 :`G` 0.785926 :`B` 1.0 :`A` 1.0) :`NewEnumerator1` (struct :`R` 1.0 :`G` 1.0 :`B` 1.0 :`A` 1.0) :!type "LinearColor Structure"))))

(fn `AddBuff`
  (params (Buff :type "/Game/Characters/Structs/Struct_Buff Structure"))
  (`KismetArrayLibrary.Array_Add` (`self.Buffs`) Buff)
  (`self.Buff Added` Buff))

(fn `GetTotalBuffValue`
  (params (Type :type "/Game/Characters/Structs/ENUM_BuffType Enum" :default "NewEnumerator0"))
  (returns (Value :type "Float (double-precision)"))
  (locals (Summary :type "Float (double-precision)"))
  (for _array_element (`self.Buffs`)
    (set `local.Summary` (+ (`.Value_6_C80E08AD4C7D3B05C3CF07AB1C77D9C0` (break `/Game/Characters/Structs/Struct_Buff` _array_element)) (`local.Summary`))))
  (return (`local.Summary`)))

(fn `RemoveBuff`
  (params (Buff :type "/Game/Characters/Structs/Struct_Buff Structure (by ref)"))
  (`KismetArrayLibrary.Array_RemoveItem` (`self.Buffs`) Buff)
  (`self.Buff Removed` Buff))