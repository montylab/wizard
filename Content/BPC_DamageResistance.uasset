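; BPC_DamageResistance is a component that reduces incoming damage by flat block and fractional resistance.
; CalcReceivingDamage subtracts BlockOverall, then scales by overall resistance for physical types or a per-type map lookup for magical ones, clamping at zero.
; It also returns whether damage remains; unknown types print an error and pass damage through, flagged false.
; Add functions accumulate resistances, but AddResistanceToAllMagic raises ResPhysical, which the calculation never reads.
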(fn `AddResistanceToAll`
  (params (InputPin :type "Float (double-precision)"))
  (set `self.Res_Overlall` (+ InputPin (`self.Res_Overlall`))))

(fn `AddResistanceToAllMagic`
  (params (Value :type "Float (double-precision)"))
  (set `self.Res_Physical` (+ Value (`self.Res_Physical`))))

(fn `AddResistanceToMagic`
  (params (Resistance :type "/Game/Characters/Damages/ENUM_MagicType Enum" :default "NewEnumerator0") (Value :type "Float (double-precision)"))
  (`BlueprintMapLibrary.Map_Add` (`self.ResistanceToMagic`) Resistance (+ (`BlueprintMapLibrary.Map_Find` (`self.ResistanceToMagic`) Resistance) Value)))

(fn `AddResistanceToPhysical`
  (params (Value :type "Float (double-precision)"))
  (set `self.Res_Physical` (+ Value (`self.Res_Physical`))))

(fn `CalcReceivingDamage`
  (params (Damage :type "Float (double-precision)") (DamageType :type "DamageType Class Reference"))
  (returns (DamageReceiving :type "Float (double-precision)") (`Damage > 0` :type Boolean))
  (bind _returnvalue (`KismetMathLibrary.FMax` (* (- (`local.Damage`) (`self.Block_Overall`)) (- 1.0 (`self.Res_Overlall`)))))
  (castclass `/Game/Characters/Damages/BP_DamageTypePhysical` DamageType
    (:`then`
      (return _returnvalue (> _returnvalue 0.0)))
    (:`CastFailed`
      (bind _asbp_damage_type_magical (castclass `/Game/Characters/Damages/BP_DamageTypeMagical` (`local.DamageType`))
        (:`then`
          (bind _returnvalue_2 (`KismetMathLibrary.FMax` (* (- (`local.Damage`) (`self.Block_Overall`)) (- 1.0 (`BlueprintMapLibrary.Map_Find` (`self.ResistanceToMagic`) (defaults `Object` _asbp_damage_type_magical))))))
          (return _returnvalue_2 (> _returnvalue_2 0.0)))
        (:`CastFailed`
          (`KismetSystemLibrary.PrintString` "No Damage Type Class Found" true true (struct :`R` 1.0 :`B` 0.033923 :`A` 1.0))
          (return (`local.Damage`) false))))))