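; BP_MagicCrystalTotem is a damageable crystal totem whose crystal material is set from CrystalType in the Construction Script.
; Damage passes through a resistance component into a health component, whose changes update a child-actor healthbar.
; On death, Explode enables crystal physics and applies radial impulses from the rock, then repeats via a short timer.
; GetHealth returns a constant zero, and hit effects, stun and destroy logic are unconnected.
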(event `self.ReceiveBeginPlay`
  (bind _bpc_healthcomponent (`self.BPC_HealthComponent`))
  ; Save casted Healthbar
  (bind _asbp_healthbar (cast `/Game/Enemies/Components/BP_Healthbar` (`ChildActorComponent.ChildActor` (`self.BP_Healthbar`))))
  (set `self.As BP Healthbar` _asbp_healthbar)
  (`/Game/Enemies/Components/BP_Healthbar.Initialize` (`self.As BP Healthbar`) (`/Game/Enemies/Components/BPC_HealthComponent.Health` _bpc_healthcomponent) (`/Game/Enemies/Components/BPC_HealthComponent.MaxHealth` _bpc_healthcomponent)))

(event `self.ReceiveAnyDamage`
  (params (Damage :type "Float (single-precision)") (DamageType :type "DamageType Object Reference") (InstigatedBy :type "Controller Object Reference") (DamageCauser :type "Actor Object Reference"))
  (`/Game/Enemies/Components/BPC_HealthComponent.TakeDamage` (`self.BPC_HealthComponent`) (`/Game/BPC_DamageResistance.CalcReceivingDamage` (`self.BPC_DamageResistance`) Damage (`GameplayStatics.GetObjectClass` DamageType)) InstigatedBy DamageCauser)
  (`KismetSystemLibrary.PrintString` "Damaged!"))

(event `self.BPC_HealthComponent.OnHealthChanged`
  (params (Health :type "Float (double-precision)") (DeltaHealth :type "Float (double-precision)") (CauserController :type "Controller Object Reference") (CauserActor :type "Actor Object Reference"))
  (set `self.Last Damage` DeltaHealth)
  (if (> DeltaHealth 0.0)
    (`/Game/Enemies/Components/BP_Healthbar.TakeDamage` (`self.As BP Healthbar`) DeltaHealth)
    (else
      (`/Game/Enemies/Components/BP_Healthbar.RestoreHealth` (`self.As BP Healthbar`) DeltaHealth))))

(event `self.BPC_HealthComponent.OnDied`
  (params (CauserController :type "Controller Object Reference") (CauserActor :type "Actor Object Reference"))
  (`self.Die` CauserController CauserActor))

(fn `Die`
  (params (DeathCauserController :type "Controller Object Reference") (DeathCauserActor :type "Actor Object Reference"))
  (`self.Explode`)
  (`KismetSystemLibrary.K2_SetTimer` null "Explode" 0.01 false true 0.01 0.01)
  (return))

(fn `Explode`
  (`PrimitiveComponent.SetCollisionEnabled` (`self.stylized_rock`) "NoCollision")
  (for _array_element (`SceneComponent.GetChildrenComponents` (`self.Crystals`) true)
    (bind _asstatic_mesh_component (cast `StaticMeshComponent` _array_element))
    (`PrimitiveComponent.SetSimulatePhysics` _asstatic_mesh_component true)
    (`PhysicsObjectBlueprintLibrary.ApplyRadialImpulse` _asstatic_mesh_component (`SceneComponent.K2_GetComponentLocation` (`self.stylized_rock`)) 5000.0 10000.0 "RIF_Constant"))
  (`PrimitiveComponent.SetCollisionEnabled` (`self.stylized_rock`) "QueryAndPhysics"))

(fn `GetCollisionComponent`
  (returns (CollisionComponent :type "PrimitiveComponent Object Reference"))
  (return (`self.BoxCollision`)))

(fn `GetHealth`
  (returns (Health :type "Float (double-precision)"))
  (return 0.0))

(fn `UserConstructionScript`
  (for _array_element (`SceneComponent.GetChildrenComponents` (`self.Crystals`) false)
    (bind _asstatic_mesh_component (cast `StaticMeshComponent` _array_element))
    (`PrimitiveComponent.SetMaterial` _asstatic_mesh_component 0 (`BlueprintMapLibrary.Map_Find` (`self.Materials`) (`self.CrystalType`)))))