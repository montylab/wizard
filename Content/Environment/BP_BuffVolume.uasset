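; BP_BuffVolume is a trigger volume that grants buffs to actors while they are inside it.
; On begin overlap, its box collision adds every entry in the Buffs array to the actor's BPC_Buffs component, and on end overlap removes them.
; The construction script fits the box to the linked PostProcessVolumeAttached, copying its location and deriving the extent from its scale.
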(event `self.BoxCollision.OnComponentBeginOverlap`
  (params (OverlappedComponent :type "PrimitiveComponent Object Reference") (OtherActor :type "Actor Object Reference") (OtherComp :type "PrimitiveComponent Object Reference") (OtherBodyIndex :type Integer) (bFromSweep :type Boolean) (SweepResult :type "HitResult Structure (by ref)"))
  (bind _returnvalue (`self.GetComponentByClass` OtherActor "/Game/Characters/BP_Components/BPC_Buffs.BPC_Buffs_C"))
  (`/Engine/EditorBlueprintResources/StandardMacros.IsValid` _returnvalue
    (:`Is Valid`
      (for _array_element (`self.Buffs`)
        (`/Game/Characters/BP_Components/BPC_Buffs.AddBuff` _returnvalue _array_element)))))

(event `self.BoxCollision.OnComponentEndOverlap`
  (params (OverlappedComponent :type "PrimitiveComponent Object Reference") (OtherActor :type "Actor Object Reference") (OtherComp :type "PrimitiveComponent Object Reference") (OtherBodyIndex :type Integer))
  (bind _returnvalue (`self.GetComponentByClass` OtherActor "/Game/Characters/BP_Components/BPC_Buffs.BPC_Buffs_C"))
  (`/Engine/EditorBlueprintResources/StandardMacros.IsValid` _returnvalue
    (:`Is Valid`
      (for _array_element (`self.Buffs`)
        (`/Game/Characters/BP_Components/BPC_Buffs.RemoveBuff` _returnvalue _array_element)))))

(fn `UserConstructionScript`
  (`SceneComponent.K2_SetWorldLocation` (`self.BoxCollision`) (`self.K2_GetActorLocation` (`self.PostProcessVolumeAttached`)) false false)
  (`BoxComponent.SetBoxExtent` (`self.BoxCollision`) (* (`self.GetActorScale3D` (`self.PostProcessVolumeAttached`)) 100) true))