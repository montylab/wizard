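; BP_MagicBarrier is a barrier actor that disappears when a designated actor dies.
; On BeginPlay it binds to the tracked actor's BPC_HealthComponent death event and, only if that component exists, swaps the Barrier to a dynamic material instance.
; On death, a timeline drives the DyingOpacity material parameter, then destroys the barrier.
; The construction script applies the base material to the Barrier.
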(event `self.ReceiveBeginPlay`
  (bind _actortotrackdeath (`self.ActorToTrackDeath`))
  (bind _returnvalue (`self.GetComponentByClass` _actortotrackdeath "/Game/Enemies/Components/BPC_HealthComponent.BPC_HealthComponent_C"))
  (`/Engine/EditorBlueprintResources/StandardMacros.IsValid` _actortotrackdeath
    (:`Is Valid`
      (`/Engine/EditorBlueprintResources/StandardMacros.IsValid` _returnvalue
        (:`Is Valid`
          (add `/Game/Enemies/Components/BPC_HealthComponent.OnDied` _returnvalue (delegate `onTrackedActorDied`))
          (bind _returnvalue_2 (`KismetMaterialLibrary.CreateDynamicMaterialInstance` (`self.Material`)))
          (bind _output_get (set `self.MI_Dynamic` _returnvalue_2))
          (`PrimitiveComponent.SetMaterial` (`self.Barrier`) 0 _output_get))))))

(event `onTrackedActorDied`
  (params (CauserController :type "Controller Object Reference") (CauserActor :type "Actor Object Reference"))
  (bind (_direction _normalizedsize) (`Timeline|Death opacity fade` :!via `PlayFromStart`)
    (:`Update`
      (`MaterialInstanceDynamic.SetScalarParameterValue` (`self.MI_Dynamic`) "DyingOpacity" _normalizedsize))
    (:`Finished`
      (`self.K2_DestroyActor`))))

(fn `UserConstructionScript`
  (`PrimitiveComponent.SetMaterial` (`self.Barrier`) 0 (`self.Material`)))