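; Enemy spell actor that deals purple magical damage scaled by how deeply a victim enters its box, destroying itself once its cast age reaches five seconds.
; Actors tagged for enemy spell damage enter a map on overlap; Tick records each VR pawn's peak bounds-intersection volume between camera capsule and box.
; On overlap end, damage is base damage times that peak's capped fraction of box volume.
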(event `self.ReceiveBeginPlay`
  (`parent.ReceiveBeginPlay`)
  (`self.AddCloudPoint` (+ (`self.K2_GetActorLocation`) (10.0 10.0 10.0))))

(event `self.ReceiveTick`
  (params (DeltaSeconds :type "Float (single-precision)"))
  (bind (_origin _boxextent) (`KismetSystemLibrary.GetComponentBounds` (`self.Box`)))
  (`self.Tick` DeltaSeconds)
  (if (< (`self.CastedAge`) 5.0)
    (bind _keys (`BlueprintMapLibrary.Map_Keys` (`self.OverlapMap`)))
    (for _array_element _keys
      (bind _asvrpawn (cast `/Game/Player/VRPawn` _array_element))
      (bind _output_get (set `self.temp_CharacterReceivingDamage` _asvrpawn))
      (`/Engine/EditorBlueprintResources/StandardMacros.IsValid` _output_get
        (:`Is Valid`
          (bind (_origin_2 _boxextent_2) (`KismetSystemLibrary.GetComponentBounds` (`/Game/Player/VRPawn.CameraCapsule` _asvrpawn)))
          (bind (_center _extent _volume _isoverlap) (`self.GetOverlapBoxParams` _origin_2 _boxextent_2 _origin _boxextent))
          (if _isoverlap
            (`BlueprintMapLibrary.Map_Add` (`self.OverlapMap`) (`self.temp_CharacterReceivingDamage`) (`KismetMathLibrary.FMax` _volume (`BlueprintMapLibrary.Map_Find` (`self.OverlapMap`) (`self.temp_CharacterReceivingDamage`))))))))
    (else
      (`self.K2_DestroyActor`))))

(event `self.Box.OnComponentBeginOverlap`
  (params (OverlappedComponent :type "PrimitiveComponent Object Reference") (OtherActor :type "Actor Object Reference") (OtherComp :type "PrimitiveComponent Object Reference") (OtherBodyIndex :type Integer) (bFromSweep :type Boolean) (SweepResult :type "HitResult Structure (by ref)"))
  (if (and (`self.ActorHasTag` OtherActor "CanTakeEnemySpellDamage") (not (`BlueprintMapLibrary.Map_Contains` (`self.OverlapMap`) OtherActor)))
    (`BlueprintMapLibrary.Map_Add` (`self.OverlapMap`) OtherActor)
    (`KismetSystemLibrary.PrintString` (`KismetStringLibrary.BuildString_Double` (`KismetSystemLibrary.GetDisplayName` OtherActor) " added to map"))))

(event `self.Box.OnComponentEndOverlap`
  (params (OverlappedComponent :type "PrimitiveComponent Object Reference") (OtherActor :type "Actor Object Reference") (OtherComp :type "PrimitiveComponent Object Reference") (OtherBodyIndex :type Integer))
  (bind (_value _returnvalue) (`BlueprintMapLibrary.Map_Find` (`self.OverlapMap`) OtherActor))
  (if _returnvalue
    (bind _output_get (set `self.temp_CollisionFinishActor` OtherActor))
    (`GameplayStatics.ApplyDamage` _output_get (* (`self.BaseDamage`) (`KismetMathLibrary.FMin` (/ _value (`self.GetSceneObjectVolume` (`self.Box`))) 1.0)) (`Pawn.GetController` (`self.GetInstigator`)) self "/Game/Characters/Damages/BP_DamageTypeMagical_Purple.BP_DamageTypeMagical_Purple_C")
    (`BlueprintMapLibrary.Map_Remove` (`self.OverlapMap`) (`self.temp_CollisionFinishActor`))))

(event `/Game/Debug/BPI_Debug.ChangeDebugState`
  (params (IsDebugEnabled :type Boolean))
  (`SceneComponent.SetHiddenInGame` (`self.Box`) (not IsDebugEnabled) false))

(fn `UserConstructionScript`
  (`parent.UserConstructionScript`))