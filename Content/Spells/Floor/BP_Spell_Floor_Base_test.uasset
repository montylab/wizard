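; Base floor spell actor: a ground decal with a collision sphere, audio and two components that rise, which destroys itself when its fade ends.
; BeginPlay fades a dynamic decal material's opacity in, then plays a second timeline in reverse before destruction.
; Tick raises both components at different rates up to a capped elevation; the growing size it computes never reaches the decal.
; The construction script sizes sphere and decal from Size.
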(event `self.ReceiveBeginPlay`
  (`AudioComponent.Play` (`self.AudioPlayer`) 0.0)
  (bind _returnvalue (`KismetMaterialLibrary.CreateDynamicMaterialInstance` (`DecalComponent.GetDecalMaterial` (`self.Decal`))))
  (bind _output_get (set `self.MatInstance` _returnvalue))
  (`DecalComponent.SetDecalMaterial` (`self.Decal`) _output_get)
  (bind (_direction _opacity) (`Timeline|Decal Fade in` :!via `PlayFromStart`)
    (:`Update`
      (`MaterialInstanceDynamic.SetScalarParameterValue` (`self.MatInstance`) "Opacity" _opacity))
    (:`Finished`
      (bind (_direction_2 _opacity_2) (`Timeline|Timeline` :!via `ReverseFromEnd`)
        (:`Update`
          (`MaterialInstanceDynamic.SetScalarParameterValue` (`self.MatInstance`) "Opacity" _opacity_2))
        (:`Finished`
          (`self.K2_DestroyActor`))))))

(event `self.ReceiveTick`
  (params (DeltaSeconds :type "Float (single-precision)"))
  (bind _output_get (set `self.GrowingSize` (`KismetMathLibrary.FMin` (+ (* DeltaSeconds (`self.GrowSpeed`)) (`self.GrowingSize`)) (`self.MaxSize`))))
  (bind _output_get_2 (set `self.Elevation` (`KismetMathLibrary.FMin` (+ (* DeltaSeconds (`self.ElevatitonSpeed`)) (`self.Elevation`)) (`self.ElevationEnd`))))
  (`SceneComponent.K2_SetRelativeLocation` (`self.FromTheGround`) (`KismetMathLibrary.MakeVector` 0.0 0.0 _output_get_2) false false)
  (`SceneComponent.K2_SetRelativeLocation` (`self.FromTheGround2`) (`KismetMathLibrary.MakeVector` 0.0 0.0 (+ (* (`self.Elevation`) 5.0) -100.0)) false false))

(fn `UserConstructionScript`
  (bind _size (`self.Size`))
  (`SphereComponent.SetSphereRadius` (`self.CollisionSphere`) (/ _size 2.0) true)
  (`SceneComponent.SetWorldScale3D` (`self.Decal`) (`KismetMathLibrary.Conv_DoubleToVector` (/ _size 2.0))))