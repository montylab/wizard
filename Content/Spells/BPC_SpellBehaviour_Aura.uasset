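; Spell behaviour component for the Aura spell, which expands the spell object's point cloud and then leaves an aura actor behind.
; Each tick scales the cloud points outward by the spell's speed, removes those beyond a fixed radius, and refreshes the Niagara parameters and collision box.
; Once the spell's cast age passes a threshold, it spawns BP_Aura at the launch point, latches a destroy flag and destroys the spell object after a delay.
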(event `self.ReceiveBeginPlay`
  (`parent.ReceiveBeginPlay`))

(event `self.ReceiveTick`
  (params (DeltaSeconds :type "Float (single-precision)"))
  (`self.Move` DeltaSeconds)
  (bind _should_destroy_ (`self.CheckIfShouldDestroy`))
  (if _should_destroy_
    (`KismetSystemLibrary.Delay` 5.0)
    (`Actor.K2_DestroyActor` (`self.SpellObject`))))

(fn `CheckIfShouldDestroy`
  (returns (`Should Destroy?` :type Boolean))
  (if (`self.ShouldDestroy`)
    (return true)
    (elif (> (`/Game/Spells/BP_Spell.CastedAge` (`self.SpellObject`)) 5.0)
      (`|SpawnActorFromClass` "/Game/Spells/BP_Aura.BP_Aura_C" (`KismetMathLibrary.Conv_VectorToTransform` (`/Game/Spells/BP_Spell.LaunchPoint` (`self.SpellObject`))) "AlwaysSpawn" "MultiplyWithRoot" null 100.0 null)
      (bind _output_get (set `self.ShouldDestroy` true))
      (return _output_get))))

(fn `Move`
  (params (DeltaSeconds :type "Float (double-precision)"))
  (locals (OffsetDelta :type "Float (double-precision)"))
  (bind _spellobject (`self.SpellObject`))
  (set `local.OffsetDelta` (* DeltaSeconds (`/Game/Spells/BP_Spell.Speed` (`self.SpellObject`))))
  (for (_array_element _array_index) (`/Game/Spells/BP_Spell.Cloud` (`self.SpellObject`))
    (bind _returnvalue (* _array_element (+ (/ (`local.OffsetDelta`) 1000.0) 1.0)))
    (if (> (`KismetMathLibrary.VSize` _returnvalue) 300.0)
      (`KismetArrayLibrary.Array_Remove` (`/Game/Spells/BP_Spell.Cloud` (`self.SpellObject`)) _array_index)
      (else
        (`KismetArrayLibrary.Array_Set` (`/Game/Spells/BP_Spell.Cloud` (`self.SpellObject`)) _array_index _returnvalue))))
  (`/Game/Spells/BP_Spell.UpdateNiagaraParams` _spellobject)
  (`/Game/Spells/BP_Spell.UpdateCollisionBox` _spellobject))