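; Ground crawler spell actor that animates a growing decal and two components rising from the ground.
; Tick increases a size value up to a cap and applies it to the decal's scale, with X held to at most 1.
; It also raises an elevation value up to an end height, driving both components' relative Z, the second from a lower offset at five times the rate.
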(event `self.ReceiveTick`
  (params (DeltaSeconds :type "Float (single-precision)"))
  (bind _output_get (set `self.Size` (`KismetMathLibrary.FMin` (+ (* DeltaSeconds (`self.GrowSpeed`)) (`self.Size`)) (`self.MaxSize`))))
  (bind (_returnvalue_x _returnvalue_y _returnvalue_z) (`KismetMathLibrary.BreakVector` (`KismetMathLibrary.Conv_DoubleToVector` _output_get)))
  (`SceneComponent.SetWorldScale3D` (`self.Decal`) (`KismetMathLibrary.MakeVector` (`KismetMathLibrary.FMin` _returnvalue_x 1.0) _returnvalue_y _returnvalue_z))
  (bind _output_get_2 (set `self.Elevation` (`KismetMathLibrary.FMin` (+ (* DeltaSeconds (`self.ElevatitonSpeed`)) (`self.Elevation`)) (`self.ElevationEnd`))))
  (`SceneComponent.K2_SetRelativeLocation` (`self.FromTheGround`) (`KismetMathLibrary.MakeVector` 0.0 0.0 _output_get_2) false false)
  (`SceneComponent.K2_SetRelativeLocation` (`self.FromTheGround2`) (`KismetMathLibrary.MakeVector` 0.0 0.0 (+ (* (`self.Elevation`) 5.0) -100.0)) false false))

(fn `UserConstructionScript`)