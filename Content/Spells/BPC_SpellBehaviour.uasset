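; BPC_SpellBehaviour is an actor component that drives the motion and growth of its owning BP_Spell after casting.
; It caches the owning spell on BeginPlay and, each tick while the spell is cast, moves it along its direction at its speed without sweeping.
; The same Move step scales the root with a clamped power curve of cast age, and OnActivated is left empty.
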(event `self.ReceiveBeginPlay`
  (bind _asbp_spell (cast `/Game/Spells/BP_Spell` (`self.GetOwner`)))
  (set `self.SpellObject` _asbp_spell))

(event `self.ReceiveTick`
  (params (DeltaSeconds :type "Float (single-precision)"))
  (if (`/Game/Spells/BP_Spell.isCasted` (`self.SpellObject`))
    (`self.Move` DeltaSeconds)))

(fn `Move`
  (params (DeltaSeconds :type "Float (double-precision)"))
  (bind _spellobject (`self.SpellObject`))
  (`Actor.K2_AddActorWorldOffset` (`self.SpellObject`) (* (`/Game/Spells/BP_Spell.Speed` _spellobject) DeltaSeconds (`/Game/Spells/BP_Spell.Direction` _spellobject)) false false)
  (`SceneComponent.SetRelativeScale3D` (`Actor.RootComponent` (`self.SpellObject`)) (`KismetMathLibrary.Conv_DoubleToVector` (`KismetMathLibrary.FMin` (`KismetMathLibrary.FMax` (/ (`KismetMathLibrary.MultiplyMultiply_FloatFloat` (+ (`/Game/Spells/BP_Spell.CastedAge` (`self.SpellObject`)) 3.0) 1.3) 5.0) 1.0) 5.0))))

(fn `OnActivated`)