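; BP_Aura is a damageable protective aura spell actor with a light and a collision sphere.
; On BeginPlay it sets health to maximum and fades the light in to its original intensity through a timeline.
; Damage reduces health, and at zero it spawns a Niagara death effect and sound, then destroys itself.
; Collision sphere visibility follows the VR pawn controller's debug flag, and its overlap handler is empty.
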(event `/Game/Debug/BPI_Debug.ChangeDebugState`
  (params (IsDebugEnabled :type Boolean))
  ;[0.15 0.09666 0 0.5] Set debug state of controller
  (`self.UpdateDebugState` IsDebugEnabled))

(event `self.ReceiveBeginPlay`
  (`|ExecutionSequence`
    (:`then_0`
      ;[0.15 0.09666 0 0.5] Set debug state of controller
      (bind _asbp_vr_pawn_controller (cast `/Game/Player/BP_VR_Pawn_Controller` (`GameplayStatics.GetPlayerController` 0)))
      (`self.UpdateDebugState` (`/Game/Player/BP_VR_Pawn_Controller.IsDebugEnabled` _asbp_vr_pawn_controller)))
    (:`then_1`
      (set `self.LightsInitialIntensity` (`LightComponentBase.Intensity` (`self.AuraLight`)))
      (set `self.Health` (`self.MaxHealth`))
      (bind (_direction _intensity) (`Timeline|Lights on` :!via `PlayFromStart`)
        (:`Update`
          (`LightComponent.SetIntensity` (`self.AuraLight`) (* _intensity (`self.LightsInitialIntensity`))))))))

(event `self.ReceiveAnyDamage`
  (params (Damage :type "Float (single-precision)") (DamageType :type "DamageType Object Reference") (InstigatedBy :type "Controller Object Reference") (DamageCauser :type "Actor Object Reference"))
  (bind _returnvalue (`self.K2_GetActorLocation`))
  (bind _output_get (set `self.Health` (- (`self.Health`) Damage)))
  (if (<= _output_get 0.0)
    (`NiagaraFunctionLibrary.SpawnSystemAtLocation` "/Game/Spells/Niagara/NS_ProtectiveAuraDies.NS_ProtectiveAuraDies" _returnvalue)
    (`GameplayStatics.PlaySoundAtLocation` "/Game/Assets/Sounds/MS_Aura_Is_Blown.MS_Aura_Is_Blown" _returnvalue (struct) 1.0 1.0 0.0 null null null null)
    (`self.K2_DestroyActor`)))

(event `self.CollisionSphere.OnComponentBeginOverlap`
  (params (OverlappedComponent :type "PrimitiveComponent Object Reference") (OtherActor :type "Actor Object Reference") (OtherComp :type "PrimitiveComponent Object Reference") (OtherBodyIndex :type Integer) (bFromSweep :type Boolean) (SweepResult :type "HitResult Structure (by ref)")))

(fn `GetHealth`
  (returns (Health :type "Float (double-precision)"))
  (return 0.0))

(fn `UserConstructionScript`)