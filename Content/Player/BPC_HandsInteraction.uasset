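; VR hand-gesture component that detects spell push motions and reports them to its owning BPI_SpellCaster.
; Each tick it records both motion controllers' movement in a rolling time window, drawn as debug arrows.
; Summed shifts yield direction and speed, with thresholds rising as pushes turn away from camera forward.
; Same-tick pushes from both hands report their angle, plus an averaged double push if aligned, relying on left-then-right check order.
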(event `self.ReceiveBeginPlay`
  (bind _asbpi_spell_caster (cast `/Game/Player/BPI_SpellCaster` (`self.GetOwner`)))
  (set `self.Owner` _asbpi_spell_caster))

(event `self.ReceiveTick`
  (params (DeltaSeconds :type "Float (single-precision)"))
  (`self.Tick` DeltaSeconds)
  (set `self.isFirstHandReadyForDoublePush?` false)
  (`self.DrawDebugInfo` (`self.LeftHandPoints`))
  (`self.DrawDebugInfo` (`self.RightHandPoints`))
  (`self.CheckPush` (`self.LeftHandPoints`) true)
  (`self.CheckPush` (`self.RightHandPoints`)))

(event `SpellPush_Event`
  (params (Direction :type "Vector Structure") (IsLeftHand :type "Boolean (by ref)"))
  (bind _returnvalue (`KismetSystemLibrary.Conv_InterfaceToObject` (`self.Owner`)))
  (if IsLeftHand
    (message `/Game/Player/BPI_SpellCaster.SpellPushLeft` _returnvalue Direction 0.0)
    (else
      (message `/Game/Player/BPI_SpellCaster.SpellPushRight` _returnvalue Direction 0.0))))

(event `Spell Push Double (any hand)`
  (params (isLeftHand :type Boolean) (Direction :type "Vector Structure") (Speed :type "Float (double-precision)"))
  (bind _returnvalue (`KismetMathLibrary.Normal` Direction))
  (bind _firsthandspeed (`self.FirstHandSpeed`))
  (if (`self.isFirstHandReadyForDoublePush?`)
    (bind _angle (`self.AngleBetweenTwoVectors` (`self.FirstHandDirection`) _returnvalue))
    (message `/Game/Player/BPI_SpellCaster.SpellPushDoubleAngle` (`KismetSystemLibrary.Conv_InterfaceToObject` (`self.Owner`)) _angle (`self.FirstHandDirection`) _returnvalue _firsthandspeed Speed)
    (if (< (`KismetMathLibrary.Abs` _angle) (`self.MaxAngleForDoublePush`))
      (message `/Game/Player/BPI_SpellCaster.SpellPushDouble` (`KismetSystemLibrary.Conv_InterfaceToObject` (`self.Owner`)) (`KismetMathLibrary.Normal` (/ (+ _returnvalue (`self.FirstHandDirection`)) 2)) (/ (+ _firsthandspeed Speed) 2.0)))
    (else
      (set `self.isFirstHandReadyForDoublePush?` true)
      (set `self.FirstHandDirection` _returnvalue)
      (set `self.FirstHandSpeed` Speed))))

(fn `AngleBetweenTwoVectors`
  (params (A :type "Vector Structure") (B :type "Vector Structure"))
  (returns (Angle :type "Float (double-precision)"))
  (bind _returnvalue (`KismetMathLibrary.Normal` B))
  (bind _returnvalue_2 (`KismetMathLibrary.Normal` A))
  (bind _returnvalue_3 (`KismetMathLibrary.DegAcos` (`KismetMathLibrary.Dot_VectorVector` _returnvalue_2 _returnvalue)))
  (if (> (.z (`KismetMathLibrary.Cross_VectorVector` _returnvalue_2 _returnvalue)) 0.0)
    (return _returnvalue_3)
    (else
      (return (* _returnvalue_3 -1.0)))))

(fn `CheckPush`
  (params (Points :type "Array of /Game/Player/S_HandPointsOverTime Structure (by ref)") (isLeftHand :type Boolean))
  (locals (`Average shift` :type "Vector Structure") (`Total shift` :type "Vector Structure") (`Total time` :type "Float (double-precision)") (Direction :type "Vector Structure" :default (0.0 0.0 0.0)) (PushSpeed :type "Float (double-precision)") (ImpedeMultiplier :type "Float (double-precision)" :default 1.0) (TotalDistance :type "Float (double-precision)"))
  (`|ExecutionSequence`
    (:`then_2`
      (for _array_element (`local.Points`)
        (bind (_point _shiftvector _duration) (break `/Game/Player/S_HandPointsOverTime` _array_element))
        (set `local.Total shift` (+ _shiftvector (`local.Total shift`)))
        (set `local.Total time` (+ _duration (`local.Total time`))))
      (set `local.Average shift` (/ (`local.Total shift`) (`KismetArrayLibrary.Array_Length` (`local.Points`))))
      (set `local.Direction` (`KismetMathLibrary.Normal` (`local.Average shift`)))
      (`|ExecutionSequence`
        (:`then_0`
          ; Easy shoot forward, harder for sides, almost imposible backwards
          (bind _output_get (set `local.TotalDistance` (`KismetMathLibrary.VSize` (`local.Total shift`))))
          (if (> _output_get 15.0)
            (bind _angle (`self.AngleBetweenTwoVectors` (`local.Direction`) (`self.OwnerForwardVector`)))
            (set `local.ImpedeMultiplier` (+ 1.0 (* (`.ReturnValue` (`KismetMathLibrary.FMod` (`KismetMathLibrary.Abs` _angle) 30.0)) 0.2)))
            (else
              (return))))
        (:`then_2`
          (bind _output_get_2 (set `local.PushSpeed` (/ (`local.TotalDistance`) (`local.Total time`))))
          (if (> _output_get_2 (* (`self.DoubleSpellPushSpeed`) (`local.ImpedeMultiplier`)))
            (`self.Spell Push Double (any hand)` (`local.isLeftHand`) (`local.Direction`) (`local.PushSpeed`))
            (if (> (`local.PushSpeed`) (* (`self.SpellPushSpeed`) (`local.ImpedeMultiplier`)))
              (`self.SpellPush_Event` (`local.Direction`) (`local.isLeftHand`)))))))))

(fn `DrawDebugInfo`
  (params (Points :type "Array of /Game/Player/S_HandPointsOverTime Structure (by ref)"))
  (for _array_element Points
    (bind (_point _shiftvector _duration) (break `/Game/Player/S_HandPointsOverTime` _array_element))
    (bind _returnvalue (- 1.2 (* _duration 33.0 1.0)))
    (`KismetSystemLibrary.DrawDebugArrow` _point (+ _point _shiftvector) 0.2 (`KismetMathLibrary.MakeColor` _returnvalue _returnvalue _returnvalue 0.5) 0.0 0.1)))

(fn `GetHandsShiftDirection`
  (returns (LeftDirection :type "Vector Structure") (LeftSpeed :type "Vector Structure") (RightDirection :type "Vector Structure") (RightSpeed :type "Vector Structure"))
  (locals (RightShiftDirection :type "Vector Structure")))

(fn `Init`
  (params (`Left Hand Motion Controller` :type "MotionControllerComponent Object Reference (by ref)") (`Right Hand Motion Controller` :type "MotionControllerComponent Object Reference (by ref)"))
  (set `self.MotionControllerLeft` `Left Hand Motion Controller`)
  (set `self.MotionControllerRight` `Right Hand Motion Controller`))

(fn `Tick`
  (params (DeltaTime :type "Float (double-precision)"))
  (set `self.Age` (+ DeltaTime (`self.Age`)))
  (set `self.OwnerForwardVector` (`SceneComponent.GetForwardVector` (`/Game/Player/VRPawn.Camera` (cast `/Game/Player/VRPawn` (`self.GetOwner`) :!pure true))))
  (`self.TickHand` (`self.MotionControllerLeft`) (`local.DeltaTime`) (`self.LeftHandPoints`))
  (`self.TickHand` (`self.MotionControllerRight`) (`local.DeltaTime`) (`self.RightHandPoints`)))

(fn `TickHand`
  (params (Hand :type "MotionControllerComponent Object Reference (by ref)") (DeltaTime :type "Float (double-precision) (by ref)") (Points :type "Array of /Game/Player/S_HandPointsOverTime Structure (by ref)"))
  (locals (HandLocation :type "Vector Structure" :default (0.0 0.0 0.0)) (PrevPointLocation :type "Vector Structure"))
  (bind _returnvalue (`SceneComponent.K2_GetComponentLocation` Hand))
  (bind _points (`local.Points`))
  (bind _prevpointlocation (`local.PrevPointLocation`))
  (set `local.HandLocation` _returnvalue)
  (if (not (`KismetArrayLibrary.Array_IsEmpty` (`local.Points`)))
    (set `local.PrevPointLocation` (`.point_3_AE9006A04EFEFE6255D8C398BB702B4B` (break `/Game/Player/S_HandPointsOverTime` (`|GetArrayItem` _points (`KismetArrayLibrary.Array_LastIndex` _points))))))
  (`KismetArrayLibrary.Array_Add` (`local.Points`) (make `/Game/Player/S_HandPointsOverTime` _returnvalue (- (`local.HandLocation`) (`KismetMathLibrary.SelectVector` (`local.HandLocation`) _prevpointlocation (`KismetMathLibrary.Vector_IsZero` _prevpointlocation))) (`local.DeltaTime`) (`self.Age`)))
  ; Clear from old nodes
  (while (and (>= (`KismetArrayLibrary.Array_Length` (`local.Points`)) 0) (< (+ (`.createdTime_13_FEA5005547CF0DF1901A57ABF8BFE3FF` (break `/Game/Player/S_HandPointsOverTime` (`|GetArrayItem` (`local.Points`)))) (`self.SecondsToTrack`)) (`self.Age`)))
    (`KismetArrayLibrary.Array_Remove` (`local.Points`))))