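; Player component that lets each hand grab the most recently cast spell within a short time window and steer it while grip is held.
; On BeginPlay it binds to the owner's BPC_HandsInteraction hand-movement and quick-gesture events, re-broadcasting each through its own dispatchers.
; Hand movement guides that hand's held spell with scaled force, and a quick downward gesture triggers the spell's down effect.
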(event `self.ReceiveBeginPlay`
  (bind _output_get (set `self.Owner` (`self.GetOwner`)))
  (bind _output_get_2 (set `self.BPC_HandsInteraction` (`Actor.GetComponentByClass` _output_get "/Game/Player/BPC_HandsInteraction.BPC_HandsInteraction_C")))
  (`self.SubscribeToEvents` _output_get_2))

(event `self.ReceiveTick`
  (params (DeltaSeconds :type "Float (single-precision)")))

(event `EnhancedInput|/Game/Player/Input/Actions/IA_Grab_Left_Pressed`
  (params (ActionValue :type "Float (double-precision)") (ElapsedSeconds :type "Float (double-precision)") (TriggeredSeconds :type "Float (double-precision)") (InputAction :type "InputAction Object Reference" :default "/Game/Player/Input/Actions/IA_Grab_Left_Pressed.IA_Grab_Left_Pressed"))
  ; Grab and release spells
  (:`Triggered`
    (`/Engine/EditorBlueprintResources/StandardMacros.IsValid` (`self.Controlled Spell by Left Hand`)
      (:`Is Not Valid`
        (`/Engine/EditorBlueprintResources/StandardMacros.IsValid` (`self.LastSpell`)
          (:`Is Valid`
            (if (< (`/Game/Spells/BP_Spell.CastedAge` (`self.LastSpell`)) (`self.TimeToGradASpell`))
              (set `self.Controlled Spell by Left Hand` (`self.LastSpell`)))))))))

(event `EnhancedInput|/Game/Player/Input/Actions/IA_Grab_Left_Released`
  (params (ActionValue :type "Float (double-precision)") (ElapsedSeconds :type "Float (double-precision)") (TriggeredSeconds :type "Float (double-precision)") (InputAction :type "InputAction Object Reference" :default "/Game/Player/Input/Actions/IA_Grab_Left_Released.IA_Grab_Left_Released"))
  ; Grab and release spells
  (:`Triggered`
    (set `self.Controlled Spell by Left Hand` null)))

(event `EnhancedInput|/Game/Player/Input/Actions/IA_Grab_Right_Pressed`
  (params (ActionValue :type "Float (double-precision)") (ElapsedSeconds :type "Float (double-precision)") (TriggeredSeconds :type "Float (double-precision)") (InputAction :type "InputAction Object Reference" :default "/Game/Player/Input/Actions/IA_Grab_Right_Pressed.IA_Grab_Right_Pressed"))
  ; Grab and release spells
  (:`Triggered`
    (`/Engine/EditorBlueprintResources/StandardMacros.IsValid` (`self.Controlled Spell by Right Hand`)
      (:`Is Not Valid`
        (`/Engine/EditorBlueprintResources/StandardMacros.IsValid` (`self.LastSpell`)
          (:`Is Valid`
            (if (< (`/Game/Spells/BP_Spell.CastedAge` (`self.LastSpell`)) (`self.TimeToGradASpell`))
              (set `self.Controlled Spell by Right Hand` (`self.LastSpell`)))))))))

(event `EnhancedInput|/Game/Player/Input/Actions/IA_Grab_Right_Released`
  (params (ActionValue :type "Float (double-precision)") (ElapsedSeconds :type "Float (double-precision)") (TriggeredSeconds :type "Float (double-precision)") (InputAction :type "InputAction Object Reference" :default "/Game/Player/Input/Actions/IA_Grab_Right_Released.IA_Grab_Right_Released"))
  ; Grab and release spells
  (:`Triggered`
    (set `self.Controlled Spell by Right Hand` null)))

(event `#OnLeftHandMoved`
  (params (Direction :type "Vector Structure") (Force :type "Float (double-precision)"))
  (`self.OnLeftHandMoved` Direction Force)
  (bind _controlledspell (`self.HasControlledLeftSpellGuard`)
    (:`Is Valid`
      (`self.GuideControlledSpell` _controlledspell Direction Force))))

(event `#OnRightHandMoved`
  (params (Direction :type "Vector Structure") (Force :type "Float (double-precision)"))
  (`self.OnRightHandMoved` Direction Force)
  (bind _controlledspell (`self.HasControlledRightSpellGuard`)
    (:`Is Valid`
      (`self.GuideControlledSpell` _controlledspell Direction Force))))

(event `#OnLeftHandQuickUp`
  (`self.OnLeftHandQuickUp`))

(event `#OnLeftHandQuickDown`
  (`self.OnLeftHandQuickDown`)
  (bind _controlledspell (`self.HasControlledLeftSpellGuard`)
    (:`Is Valid`
      (`/Game/Spells/BP_Spell.TriggerDownEffect` _controlledspell))))

(event `#OnLeftHandQuickForward`
  (`self.OnLeftHandQuickForward`))

(event `#OnLeftHandQuickBackward`
  (`self.OnLeftHandQuickBackward`))

(event `#OnRightHandQuickUp`
  (`self.OnRightHandQuickUp`))

(event `#OnRightHandQuickDown`
  (`self.OnRightHandQuickDown`)
  (bind _controlledspell (`self.HasControlledRightSpellGuard`)
    (:`Is Valid`
      (`/Game/Spells/BP_Spell.TriggerDownEffect` _controlledspell))))

(event `#OnRightHandQuickForward`
  (`self.OnRightHandQuickForward`))

(event `#OnRightHandQuickBackward`
  (`self.OnRightHandQuickBackward`))

(fn `GuideControlledSpell`
  (params (Spell :type "/Game/Spells/BP_Spell Object Reference (by ref)") (Direction :type "Vector Structure") (A :type "Float (double-precision)"))
  (`/Game/Spells/BP_Spell.GuideSpell` Spell Direction (* A (`self.ForceMultiplier`))))

(fn `SetLastSpell`
  (params (LastSpell :type "/Game/Spells/BP_Spell Object Reference"))
  (set `self.LastSpell` LastSpell))

(fn `SubscribeToEvents`
  (params (`Hands Interactor` :type "/Game/Player/BPC_HandsInteraction Object Reference"))
  (`|ExecutionSequence`
    (:`then_0`
      (add `/Game/Player/BPC_HandsInteraction.OnLeftHandMoved` (`local.Hands Interactor`) (`|CreateDelegate` :!event `#OnLeftHandMoved`)))
    (:`then_1`
      (add `/Game/Player/BPC_HandsInteraction.OnRightHandMoved` (`local.Hands Interactor`) (`|CreateDelegate` :!event `#OnRightHandMoved`)))
    (:`then_2`
      (add `/Game/Player/BPC_HandsInteraction.OnLeftHandQuickUp` (`local.Hands Interactor`) (`|CreateDelegate` :!event `#OnLeftHandQuickUp`))
      (add `/Game/Player/BPC_HandsInteraction.OnLeftHandQuickDown` (`local.Hands Interactor`) (`|CreateDelegate` :!event `#OnLeftHandQuickDown`))
      (add `/Game/Player/BPC_HandsInteraction.OnLeftHandQuickForward` (`local.Hands Interactor`) (`|CreateDelegate` :!event `#OnLeftHandQuickForward`))
      (add `/Game/Player/BPC_HandsInteraction.OnLeftHandQuickBackward` (`local.Hands Interactor`) (`|CreateDelegate` :!event `#OnLeftHandQuickBackward`)))
    (:`then_3`
      (add `/Game/Player/BPC_HandsInteraction.OnRightHandQuickUp` (`local.Hands Interactor`) (`|CreateDelegate` :!event `#OnRightHandQuickUp`))
      (add `/Game/Player/BPC_HandsInteraction.OnRightHandQuickDown` (`local.Hands Interactor`) (`|CreateDelegate` :!event `#OnRightHandQuickDown`))
      (add `/Game/Player/BPC_HandsInteraction.OnRightHandQuickForward` (`local.Hands Interactor`) (`|CreateDelegate` :!event `#OnRightHandQuickForward`))
      (add `/Game/Player/BPC_HandsInteraction.OnRightHandQuickBackward` (`local.Hands Interactor`) (`|CreateDelegate` :!event `#OnRightHandQuickBackward`)))
    (:`then_4`)
    (:`then_5`)))