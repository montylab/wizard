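; Player component that captures hand-drawn spell strokes from two motion controllers supplied through Init.
; Left and right Enhanced Input actions set per-hand drawing flags and, while active, send the hand's world location to the owner through BPI_Spell_Drawer, as both general and per-hand points.
; Tick accumulates per-hand timers, which IsSafeTimePassed compares to a safe-time threshold; IsDrawInProgress reports whether either hand is drawing.
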(event `self.ReceiveBeginPlay`
  (bind _asbpi_spell_drawer (cast `/Game/Player/BPI_Spell_Drawer` (`self.GetOwner`)))
  (set `self.Owner` _asbpi_spell_drawer))

(event `self.ReceiveTick`
  (params (DeltaSeconds :type "Float (single-precision)"))
  (set `self.LeftTimeAfterDrawing` (+ DeltaSeconds (`self.LeftTimeAfterDrawing`)))
  (set `self.RightTimeAfterDrawing` (+ DeltaSeconds (`self.RightTimeAfterDrawing`))))

(event `EnhancedInput|/Game/Player/Input/Actions/IA_Spell_Draw_Left`
  (params (ActionValue :type Boolean) (ElapsedSeconds :type "Float (double-precision)") (TriggeredSeconds :type "Float (double-precision)") (InputAction :type "InputAction Object Reference" :default "/Game/Player/Input/Actions/IA_Spell_Draw_Left.IA_Spell_Draw_Left"))
  (bind _returnvalue (`SceneComponent.K2_GetComponentLocation` (`self.LeftHandMC`)))
  (bind _returnvalue_2 (`KismetSystemLibrary.Conv_InterfaceToObject` (`self.Owner`)))
  (:`Triggered`
    (bind _output_get (set `self.isLeftDrawInProgress` ActionValue :!label _label))
    (if _output_get
      (message `/Game/Player/BPI_Spell_Drawer.AddPoint` _returnvalue_2 _returnvalue)
      (message `/Game/Player/BPI_Spell_Drawer.AddPointLeft` _returnvalue_2 _returnvalue)))
  (:`Ongoing`
    (goto _label))
  (:`Canceled`
    (goto _label))
  (:`Completed`
    (goto _label)))

(event `EnhancedInput|/Game/Player/Input/Actions/IA_Spell_Draw_Right`
  (params (ActionValue :type Boolean) (ElapsedSeconds :type "Float (double-precision)") (TriggeredSeconds :type "Float (double-precision)") (InputAction :type "InputAction Object Reference" :default "/Game/Player/Input/Actions/IA_Spell_Draw_Right.IA_Spell_Draw_Right"))
  (bind _returnvalue (`SceneComponent.K2_GetComponentLocation` (`self.RightHandMC`)))
  (bind _returnvalue_2 (`KismetSystemLibrary.Conv_InterfaceToObject` (`self.Owner`)))
  (:`Triggered`
    (bind _output_get (set `self.isRightDrawInProgress` ActionValue :!label _label_2))
    (if _output_get
      (message `/Game/Player/BPI_Spell_Drawer.AddPoint` _returnvalue_2 _returnvalue)
      (message `/Game/Player/BPI_Spell_Drawer.AddPointRight` _returnvalue_2 _returnvalue)))
  (:`Ongoing`
    (goto _label_2))
  (:`Canceled`
    (goto _label_2))
  (:`Completed`
    (goto _label_2)))

(fn `Init`
  (params (`Left Hand MC` :type "MotionControllerComponent Object Reference") (`Right Hand MC` :type "MotionControllerComponent Object Reference"))
  (set `self.LeftHandMC` `Left Hand MC`)
  (set `self.RightHandMC` `Right Hand MC`))

(fn `IsDrawInProgress`
  (returns (InProgress :type Boolean))
  (return (or (`self.isLeftDrawInProgress`) (`self.isRightDrawInProgress`))))

(fn `isSafeTimePassed`
  (returns (InProgress :type Boolean))
  (return (> (`KismetMathLibrary.FMin` (`self.LeftTimeAfterDrawing`) (`self.RightTimeAfterDrawing`)) (`self.SafeTimeAfterDrawing`))))