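; BP_VR_Pawn_Controller is the VR player pawn's controller, handling debug input and pausing the game on death.
; It enables input on BeginPlay, and the enable-debug action toggles a flag that it broadcasts to every actor implementing BPI_Debug.
; WhenDied pauses the game and prints a confirmation, while the special debug action only prints a test message.
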(event `self.ReceiveBeginPlay`
  (`self.EnableInput` null))

(event `EnhancedInput|/Game/Player/Input/Actions/IA_Debug_EnableDebug`
  (params (ActionValue :type Boolean) (ElapsedSeconds :type "Float (double-precision)") (TriggeredSeconds :type "Float (double-precision)") (InputAction :type "InputAction Object Reference" :default "/Game/Player/Input/Actions/IA_Debug_EnableDebug.IA_Debug_EnableDebug"))
  (:`Triggered`
    (set `self.IsDebugEnabled` (not (`self.IsDebugEnabled`)))
    (bind _outactors (`GameplayStatics.GetAllActorsWithInterface` "/Game/Debug/BPI_Debug.BPI_Debug_C"))
    (for _array_element _outactors
      (message `/Game/Debug/BPI_Debug.ChangeDebugState` _array_element (`self.IsDebugEnabled`)))))

(event `EnhancedInput|/Game/Player/Input/Actions/IA_Debug_Special`
  (params (ActionValue :type Boolean) (ElapsedSeconds :type "Float (double-precision)") (TriggeredSeconds :type "Float (double-precision)") (InputAction :type "InputAction Object Reference" :default "/Game/Player/Input/Actions/IA_Debug_Special.IA_Debug_Special"))
  (:`Triggered`
    (`KismetSystemLibrary.PrintString` "I'm special (from player pawn contorller)" true true (struct :`G` 1.0 :`B` 0.926636 :`A` 1.0))))

(fn `UserConstructionScript`)

(fn `WhenDied`
  (`GameplayStatics.SetGamePaused` true)
  (`KismetSystemLibrary.PrintString` "Pause is set")
  (return))