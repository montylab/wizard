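; BP_BaseEnemy is a VR enemy base with health, melee attack and an experience reward on death.
; Health component events drive the healthbar, damage indicators, Niagara effects, hit stun and death, with widgets yawing toward the player camera.
; An overlap volume fills a priority map of attackable actors and, like stun, updates AI Blackboard flags.
; Death detaches the controller, removes collision and grants experience to the killing VRPawn.
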(event `self.ReceiveBeginPlay`
  (`self.SetPlayerCamera`)
  ; Save casted Healthbar
  (bind _asbp_healthbar (cast `/Game/Enemies/Components/BP_Healthbar` (`ChildActorComponent.ChildActor` (`self.BP_Healthbar`))))
  (set `self.As BP Healthbar` _asbp_healthbar)
  (`self.Set AI and Blackboard`)
  ; Setup Health Changed event
  (`self.SetupHealthLogicEvent_Event`))

(event `self.ReceiveTick`
  (params (DeltaSeconds :type "Float (single-precision)"))
  (`self.RotateWidgetsToFaceCamera`))

(event `self.ReceiveAnyDamage`
  (params (Damage :type "Float (single-precision)") (DamageType :type "DamageType Object Reference") (InstigatedBy :type "Controller Object Reference") (DamageCauser :type "Actor Object Reference"))
  (`/Game/Enemies/Components/BPC_HealthComponent.TakeDamage` (`self.BPC_HealthComponent`) Damage InstigatedBy DamageCauser))

(event `self.InRangeCollision.OnComponentBeginOverlap`
  (params (OverlappedComponent :type "PrimitiveComponent Object Reference") (OtherActor :type "Actor Object Reference") (OtherComp :type "PrimitiveComponent Object Reference") (OtherBodyIndex :type Integer) (bFromSweep :type Boolean) (SweepResult :type "HitResult Structure (by ref)"))
  (bind _returnvalue (`self.GetComponentByClass` OtherActor "/Game/Blueprints/BPC_EnemyAttackable.BPC_EnemyAttackable_C"))
  (`self.Not Dead Guard`
    (:`Not Dead`
      (`/Engine/EditorBlueprintResources/StandardMacros.IsValid` _returnvalue
        (:`Is Valid`
          (`BlueprintMapLibrary.Map_Add` (`self.AttackPriorityQueue`) OtherActor (`/Game/Blueprints/BPC_EnemyAttackable.Priority` _returnvalue))
          (set `self.IsAttackableInAttackRange` true)
          (`BlackboardComponent.SetValueAsBool` (`self.Blackboard`) (`KismetStringLibrary.Conv_StringToName` "IsAttackableInAttackRange") (`self.IsAttackableInAttackRange`) :!label _label))))))

(event `self.InRangeCollision.OnComponentEndOverlap`
  (params (OverlappedComponent :type "PrimitiveComponent Object Reference") (OtherActor :type "Actor Object Reference") (OtherComp :type "PrimitiveComponent Object Reference") (OtherBodyIndex :type Integer))
  (bind _attackpriorityqueue (`self.AttackPriorityQueue`))
  (`self.Not Dead Guard`
    (:`Not Dead`
      (`/Engine/EditorBlueprintResources/StandardMacros.IsValid` (`self.GetComponentByClass` OtherActor "/Game/Blueprints/BPC_EnemyAttackable.BPC_EnemyAttackable_C")
        (:`Is Valid`
          (`BlueprintMapLibrary.Map_Remove` _attackpriorityqueue OtherActor)
          (set `self.IsAttackableInAttackRange` (not (`BlueprintMapLibrary.Map_IsEmpty` _attackpriorityqueue)))
          (goto _label))))))

(event `/Game/Debug/BPI_Debug.ChangeDebugState`
  (params (IsDebugEnabled :type Boolean))
  (bind _capsulecomponent (`self.CapsuleComponent`))
  (bind _output_get (set `self.Is Debug Enabled` IsDebugEnabled))
  (`/Engine/EditorBlueprintResources/StandardMacros.IsValid` _capsulecomponent
    (:`Is Valid`
      (bind _returnvalue (not _output_get))
      (`SceneComponent.SetHiddenInGame` _capsulecomponent _returnvalue false)
      (`SceneComponent.SetHiddenInGame` (`self.InRangeCollision`) _returnvalue false))))

(event `HealthChanged_Event`
  (params (Health :type "Float (double-precision)") (DeltaHealth :type "Float (double-precision)") (CauserController :type "Controller Object Reference") (CauserActor :type "Actor Object Reference"))
  (set `self.LastDamage` DeltaHealth)
  (if (> DeltaHealth 0.0)
    (`/Game/Enemies/Components/BP_Healthbar.TakeDamage` (`self.As BP Healthbar`) DeltaHealth)
    (bind _returnvalue (`NiagaraFunctionLibrary.SpawnSystemAttached` (`self.NS_Hit`) (`self.Mesh`) "None" (0.0 0.0 0.0) (struct) "KeepRelativeOffset" true))
    (`NiagaraComponent.SetVariableFloat` _returnvalue "ParticleCountMultiplier" (/ (`self.LastDamage`) (`/Game/Enemies/Components/BPC_HealthComponent.MaxHealth` (`self.BPC_HealthComponent`))))
    ; Spawn and Attach Damage Value Effect
    (bind _returnvalue_2 (`|SpawnActorFromClass` "/Game/Enemies/Components/BP_DamageIndicator.BP_DamageIndicator_C" (`KismetMathLibrary.MakeTransform` (0.0 0.0 0.0)) "Undefined" "MultiplyWithRoot" null (`self.LastDamage`) null))
    (`self.K2_AttachToComponent` _returnvalue_2 (`self.WidgetsContainer`) "None" "KeepRelative" "KeepRelative" "KeepRelative" true)
    (bind _output_get (set `self.IsDead` (<= (`/Game/Enemies/Components/BPC_HealthComponent.Health` (`self.BPC_HealthComponent`)) 0.0)))
    (if (not _output_get)
      ; Stunned Montage
      (bind _output_get_2 (set `self.isStunned` true))
      (`BlackboardComponent.SetValueAsBool` (`self.Blackboard`) (`KismetStringLibrary.Conv_StringToName` "IsStunned") _output_get_2)
      (`|PlayMontage` (`self.Mesh`) (`self.AM_Hit/Death`) 1.0 0.0 "Hit"
        (:`OnNotifyBegin`
          (bind _output_get_3 (set `self.isStunned` false))
          (`BlackboardComponent.SetValueAsBool` (`self.Blackboard`) (`KismetStringLibrary.Conv_StringToName` "IsStunned") _output_get_3))))
    (else
      (`/Game/Enemies/Components/BP_Healthbar.RestoreHealth` (`self.As BP Healthbar`) DeltaHealth))))

(event `SetupHealthLogicEvent_Event`
  (bind _bpc_healthcomponent (`self.BPC_HealthComponent`))
  (add `/Game/Enemies/Components/BPC_HealthComponent.OnHealthChanged` (`self.BPC_HealthComponent`) (delegate `HealthChanged_Event`))
  (add `/Game/Enemies/Components/BPC_HealthComponent.OnDied` (`self.BPC_HealthComponent`) (delegate `OnDied_Event`))
  (`/Game/Enemies/Components/BP_Healthbar.Initialize` (`self.As BP Healthbar`) (`/Game/Enemies/Components/BPC_HealthComponent.Health` _bpc_healthcomponent) (`/Game/Enemies/Components/BPC_HealthComponent.MaxHealth` _bpc_healthcomponent)))

(event `OnDied_Event`
  (params (CauserController :type "Controller Object Reference") (CauserActor :type "Actor Object Reference"))
  (`self.Die` CauserController CauserActor))

(fn `AttackMelee`
  (bind (_origin _boxextent) (`KismetSystemLibrary.GetComponentBounds` null))
  (if (`self.Is Debug Enabled`)
    (`KismetSystemLibrary.DrawDebugBox` _origin _boxextent (struct :`R` 1.0 :`B` 0.017232 :`A` 1.0) (struct) 2.0 0.5))
  (`self.PlayAnimMontage` (`self.AM_Attack`)))

(fn `Die`
  (params (DeathCauserController :type "Controller Object Reference") (DeathCauserActor :type "Actor Object Reference"))
  (bind _inrangecollision (`self.InRangeCollision`))
  (bind _capsulecomponent (`self.CapsuleComponent`))
  (`KismetSystemLibrary.PrintString` "Die!")
  (set `self.IsDead` true)
  (`self.PlayAnimMontage` (`self.AM_Hit/Death`) 1.0 "Death")
  (`self.DetachFromControllerPendingDestroy`)
  (`PrimitiveComponent.SetCollisionEnabled` _capsulecomponent "NoCollision")
  (`ActorComponent.K2_DestroyComponent` _capsulecomponent)
  (`PrimitiveComponent.SetCollisionEnabled` _inrangecollision "NoCollision")
  (`ActorComponent.K2_DestroyComponent` _inrangecollision)
  (`NiagaraFunctionLibrary.SpawnSystemAttached` (`self.NS_Death`) (`self.Mesh`) "None" (0.0 0.0 0.0) (struct) "KeepRelativeOffset" true)
  (`self.ShowExperience`)
  (bind _asvrpawn (cast `/Game/Player/VRPawn` (`Controller.K2_GetPawn` (`local.DeathCauserController`))))
  (`/Game/Player/VRPawn.AddExperience` _asvrpawn (`self.ExperienceAfterDeath`)))

(fn `RotateWidgetsToFaceCamera`
  (bind (_returnvalue_roll _returnvalue_pitch _returnvalue_yaw) (`KismetMathLibrary.BreakRotator` (`KismetMathLibrary.FindLookAtRotation` (`SceneComponent.K2_GetComponentLocation` (`self.Mesh`)) (`SceneComponent.K2_GetComponentLocation` (`self.PlayerCamera`)))))
  (`SceneComponent.K2_SetWorldRotation` (`self.WidgetsContainer`) (`KismetMathLibrary.MakeRotator` 0.0 0.0 _returnvalue_yaw) false true))

(fn `Set AI and Blackboard`
  (bind _asaicontroller (cast `AIController` (`self.GetController`)))
  (set `self.As AIController` _asaicontroller)
  (set `self.Blackboard` (`AIBlueprintHelperLibrary.GetBlackboard` _asaicontroller)))

(fn `SetPlayerCamera`
  (bind _asvrpawn (cast `/Game/Player/VRPawn` (`GameplayStatics.GetPlayerPawn` 0)))
  (set `self.PlayerCamera` (`/Game/Player/VRPawn.Camera` _asvrpawn)))

(fn `ShowExperience`
  (bind _aswbp_enemy_exp (cast `/Game/Enemies/Widgets/WBP_Enemy_Exp` (`WidgetComponent.GetWidget` (`self.Experience Count Widget`))))
  (`/Game/Enemies/Widgets/WBP_Enemy_Exp.ShowExperience` _aswbp_enemy_exp (`self.ExperienceAfterDeath`) 3.0))

(fn `UserConstructionScript`)