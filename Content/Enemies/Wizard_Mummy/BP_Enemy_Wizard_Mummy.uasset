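; Wizard mummy enemy Blueprint that damages actors tagged Attackable through an attack touch collision and carries a ranged attack component.
; The collision starts disabled, is toggled through SetAttackCollision, and switches itself off after landing a hit.
; A not-dead guard gates hits and the debug box on Tick, and construction passes the mesh to the ranged attack component for animation.
; Patrol-point blackboard setup is present but disconnected.
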(event `self.ReceiveBeginPlay`
  (`parent.ReceiveBeginPlay`)
  ; Initial disable attack collsition
  (`self.SetAttackCollisionFunc` false))

(event `self.ReceiveTick`
  (params (DeltaSeconds :type "Float (single-precision)"))
  (bind (_origin _boxextent) (`KismetSystemLibrary.GetComponentBounds` null))
  (bind _attacktouchcollision (`self.AttackTouchCollision`))
  (`parent.ReceiveTick` DeltaSeconds)
  (`self.Not Dead Guard`
    (:`Not Dead`
      ;[0.15 0.1199 0 0.5] Debug
      (if (`self.Is Debug Enabled`)
        (`KismetSystemLibrary.DrawDebugBox` _origin _boxextent (make `LinearColor` (`KismetMathLibrary.Conv_IntToDouble` (* (`KismetMathLibrary.Conv_BoolToInt` (`PrimitiveComponent.K2_IsCollisionEnabled` _attacktouchcollision)) 255))) (`SceneComponent.K2_GetComponentRotation` _attacktouchcollision) 0.0 0.2)))))

(event `self.AttackTouchCollision.OnComponentBeginOverlap`
  (params (OverlappedComponent :type "PrimitiveComponent Object Reference") (OtherActor :type "Actor Object Reference") (OtherComp :type "PrimitiveComponent Object Reference") (OtherBodyIndex :type Integer) (bFromSweep :type Boolean) (SweepResult :type "HitResult Structure (by ref)"))
  (`self.Not Dead Guard`
    (:`Not Dead`
      (if (`self.ActorHasTag` OtherActor "Attackable")
        (`GameplayStatics.ApplyDamage` OtherActor (`self.BaseDamage`) (`self.GetController` self) self)
        (`self.SetAttackCollisionFunc` false)))))

(event `self.SetAttackCollision`
  (params (`Is Enabled` :type Boolean))
  (`self.SetAttackCollisionFunc` `Is Enabled`))

(fn `SetAttackCollisionFunc`
  (params (IsEnabled :type Boolean))
  (bind _attacktouchcollision (`self.AttackTouchCollision`))
  (if IsEnabled
    (`PrimitiveComponent.SetCollisionEnabled` _attacktouchcollision "QueryOnly")
    (else
      (`PrimitiveComponent.SetCollisionEnabled` _attacktouchcollision "NoCollision"))))

(fn `UserConstructionScript`
  (set `/Game/Enemies/Components/BPC_EnemyRangedAttack.MeshToAnimate` (`self.Mesh`) (`self.BPC_EnemyRangedAttack`)))