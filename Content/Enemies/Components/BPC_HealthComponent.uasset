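; Health component for enemies that tracks current health and reports damage and death.
; Health starts at MaxHealth on BeginPlay.
; TakeDamage lowers Health, clamped at zero, and fires OnHealthChanged with the damage value, instigating controller and causing actor.
; When Health reaches zero it fires OnDied once, since further damage is ignored.
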(event `self.ReceiveBeginPlay`
  (set `self.Health` (`self.MaxHealth`)))

(fn `TakeDamage`
  (params (DamageValue :type "Float (double-precision)") (CauserController :type "Controller Object Reference") (CauserActor :type "Actor Object Reference"))
  (if (> (`self.Health`) 0.0)
    (bind _output_get (set `self.Health` (`KismetMathLibrary.FMax` (- (`self.Health`) DamageValue))))
    (`self.OnHealthChanged` _output_get (`local.DamageValue`) (`local.CauserController`) (`local.CauserActor`))
    (if (<= (`self.Health`) 0.0)
      (`self.OnDied` (`local.CauserController`) (`local.CauserActor`)))))