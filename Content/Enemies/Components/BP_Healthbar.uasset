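; BP_Healthbar is an enemy health bar Blueprint that stores health values and shows them through a WBP_Healthbar in its HealthbarWidget component.
; TakeDamage lowers health, floored at zero, and passes remaining health and applied damage to the widget as fractions of maximum.
; Initialize sets both values and refreshes the bar through a zero-damage hit.
; RestoreHealth sets health to current plus restored minus maximum, without updating the widget.
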(event `self.ReceiveBeginPlay`
  (bind _aswbp_healthbar (cast `/Game/Enemies/Widgets/WBP_Healthbar` (`WidgetComponent.GetWidget` (`self.HealthbarWidget`))))
  (set `self.As WBP_Healthbar` _aswbp_healthbar))

(fn `Initialize`
  (params (Health :type "Float (double-precision)") (MaxHealth :type "Float (double-precision)" :default 1.0))
  (set `self.Health` Health)
  (set `self.MaxHealth` MaxHealth)
  (`self.TakeDamage` 0.0))

(fn `RestoreHealth`
  (params (RestoredValue :type "Float (double-precision)"))
  (set `self.Health` (- (+ RestoredValue (`self.Health`)) (`self.MaxHealth`))))

(fn `TakeDamage`
  (params (DamageValue :type "Float (double-precision)"))
  (set `self.Health` (`KismetMathLibrary.FMax` (- (`self.Health`) DamageValue)))
  (bind _aswbp_healthbar (cast `/Game/Enemies/Widgets/WBP_Healthbar` (`WidgetComponent.GetWidget` (`self.HealthbarWidget`))))
  (`/Game/Enemies/Widgets/WBP_Healthbar.TakeDamage` _aswbp_healthbar (/ (`self.Health`) (`self.MaxHealth`)) (/ (`local.DamageValue`) (`self.MaxHealth`))))

(fn `UserConstructionScript`)