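; BP_DamageIndicator is a short-lived actor that shows a damage value through a WBP_Enemy_Damage widget.
; On BeginPlay it copies Value into the widget, then picks a random direction scaled to a fixed distance.
; A timeline curve moves the DamageTakenWidget component along that offset in relative space, and the actor destroys itself when the timeline finishes.
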(event `self.ReceiveBeginPlay`
  (bind _aswbp_enemy_damage (cast `/Game/Enemies/Widgets/WBP_Enemy_Damage` (`WidgetComponent.GetWidget` (`self.DamageTakenWidget`))))
  (set `/Game/Enemies/Widgets/WBP_Enemy_Damage.Damage` (`self.Value`) _aswbp_enemy_damage)
  (set `self.Direction` (* (`KismetMathLibrary.RandomUnitVector`) 60))
  (bind (_direction _curve) (`Timeline|Timeline` :!via `PlayFromStart`)
    (:`Update`
      (`SceneComponent.K2_SetRelativeLocation` (`self.DamageTakenWidget`) (* _curve (`self.Direction`)) false false))
    (:`Finished`
      (`self.K2_DestroyActor`))))

(event `self.ReceiveTick`
  (params (DeltaSeconds :type "Float (single-precision)")))

(fn `UserConstructionScript`)