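; Enemy actor component that performs a ranged spell attack on a given target when its RangedAttack event is called.
; It plays the ranged attack montage at half speed on the assigned mesh and waits for the Cast Start notify.
; On that notify it spawns a BP_Enemy_Spell at the owner's transform and pushes it toward the target's current location at a fixed speed.
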(event `RangedAttack`
  (params (TargetActor :type "Actor Object Reference"))
  (bind _returnvalue (`self.GetOwner`))
  (set `self.Target Actor` TargetActor)
  (bind _notifyname (`|PlayMontage` (`self.MeshToAnimate`) (`self.RangedAttackMontage`) 0.5)
    (:`OnNotifyBegin`
      (switch `name` _notifyname
        (:`CastStart`
          (bind _returnvalue_2 (`|SpawnActorFromClass` "/Game/Spells/BP_Enemy_Spell.BP_Enemy_Spell_C" (`Actor.GetTransform` _returnvalue) "Undefined" "MultiplyWithRoot" _returnvalue (cast `Pawn` _returnvalue :!pure true)))
          (`/Game/Spells/BP_Spell.Push` _returnvalue_2 (`KismetMathLibrary.Normal` (- (`Actor.K2_GetActorLocation` (`self.Target Actor`)) (`Actor.K2_GetActorLocation` (`self.GetOwner`)))) 300.0))))))