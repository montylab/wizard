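; BP_SpawnPoint is an enemy spawner that creates instances of a configured enemy class at its own transform and hands each one its patrol route.
; Tick fires spawns on an interval scaled by curves over spawner age and player distance, capped by alive and total limits.
; Patrol points convert to world space at BeginPlay, children can be detached from the alive list, and the spawner destroys itself once the total limit is reached.
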(event `self.ReceiveBeginPlay`
  (`|ExecutionSequence`
    (:`then_0`
      ; Adjust patrol points to global space
      (for (_array_element _array_index) (`self.PatrolLocations`)
        (`KismetArrayLibrary.Array_Set` (`self.PatrolLocations`) _array_index (+ _array_element (`SceneComponent.K2_GetComponentLocation` (`self.DefaultSceneRoot`))))))
    (:`then_1`
      ; Spawn actor on begin
      (if (`self.SpawnOnBegin`)
        (`self.Spawn`)))))

(event `self.ReceiveTick`
  (params (DeltaSeconds :type "Float (single-precision)"))
  (set `self.Age` (+ DeltaSeconds (`self.Age`)))
  (bind _output_get (set `self.Timer` (+ DeltaSeconds (`self.Timer`))))
  (if (>= _output_get (/ (`self.SecondsBetweenSpawns`) (`CurveFloat.GetFloatValue` (`self.SpawnFrequencyCurve`) (`self.Age`)) (+ (`CurveFloat.GetFloatValue` (`self.SpawnPlayerProximityFrequencyCurve`) (`KismetMathLibrary.Vector_Distance` (`self.K2_GetActorLocation` (`GameplayStatics.GetPlayerPawn` 0)) (`self.K2_GetActorLocation`))) 1e-05)))
    (`self.Spawn`)))

(fn `DetachChild`
  (params (Child :type "/Game/Enemies/BP_BaseEnemy Object Reference"))
  (`KismetArrayLibrary.Array_RemoveItem` (`self.SpawnedChildren`) Child))

(fn `Spawn`
  (if (< (`self.TotalSpawnedInstances`) (`self.LimitTotalSpawned`))
    (if (< (`KismetArrayLibrary.Array_Length` (`self.SpawnedChildren`)) (`self.LimitAliveSpawned`))
      (set `self.Timer` 0.0)
      (`/Engine/EditorBlueprintResources/StandardMacros.IncrementInt` (`self.TotalSpawnedInstances`)
        (:`  `
          (bind _returnvalue (`|SpawnActorFromClass` (`self.SpawningEnemiesBP`) (`self.GetTransform`) "AdjustIfPossibleButAlwaysSpawn" "MultiplyWithRoot" null self null))
          (`KismetArrayLibrary.Array_Add` (`self.SpawnedChildren`) _returnvalue)
          (`/Game/Enemies/BP_BaseEnemy.SetupPatrolPoints` _returnvalue (`self.PatrolLocations`)))))
    (else
      (`self.K2_DestroyActor`))))

(fn `UserConstructionScript`)