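; Big Guy enemy Blueprint that adds a melee attack hitbox on top of its parent class.
; AttackTouchBox collision starts disabled and is toggled through the SetAttackCollision event, which nothing in this file calls.
; While the enemy is alive, an overlap with an actor tagged Attackable applies BaseDamage and immediately disables the box, ending that hit window after one successful hit.
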(event `self.ReceiveBeginPlay`
  (`parent.ReceiveBeginPlay`)
  ; Initial disable attack collsition
  (`self.SetAttackCollisionFunc` false))

(event `self.AttackTouchBox.OnComponentBeginOverlap`
  (params (OverlappedComponent :type "PrimitiveComponent Object Reference") (OtherActor :type "Actor Object Reference") (OtherComp :type "PrimitiveComponent Object Reference") (OtherBodyIndex :type Integer) (bFromSweep :type Boolean) (SweepResult :type "HitResult Structure (by ref)"))
  (`self.Not Dead Guard`
    (:`Not Dead`
      (if (`self.ActorHasTag` OtherActor "Attackable")
        (`GameplayStatics.ApplyDamage` OtherActor (`self.BaseDamage`) (`self.GetController` self) self)
        (`self.SetAttackCollisionFunc` false)))))

(event `/Game/Enemies/BPI_Enemy_Melee_Attacker.SetAttackCollision`
  (params (`Is Enabled` :type Boolean))
  (`self.SetAttackCollisionFunc` `Is Enabled`))

(fn `SetAttackCollisionFunc`
  (params (IsEnabled :type Boolean))
  (bind _attacktouchbox (`self.AttackTouchBox`))
  (if IsEnabled
    (`PrimitiveComponent.SetCollisionEnabled` _attacktouchbox "QueryOnly")
    (else
      (`PrimitiveComponent.SetCollisionEnabled` _attacktouchbox "NoCollision"))))

(fn `UserConstructionScript`
  (`parent.UserConstructionScript`))