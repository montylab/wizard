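; Patrol path actor for enemies that defines a looping route from the points of a spline.
; The construction script caches each spline point's world location in an array.
; Query functions return the first point, the point nearest a location by squared distance, or the next point after an index, wrapping to the start.
; A debug event toggles the spline's in-game visibility.
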(event `/Game/Debug/BPI_Debug.ChangeDebugState`
  (params (IsDebugEnabled :type Boolean))
  (bind _output_get (set `self.Is Debug Enabled` IsDebugEnabled))
  (`SceneComponent.SetHiddenInGame` (`self.Spline_route`) (not _output_get) false))

(fn `GetClosestPoint`
  (params (Point :type "Vector Structure"))
  (returns (Location :type "Vector Structure") (Index :type Integer))
  (locals (MinDistanceSquared :type "Float (double-precision)" :default 999999999999.0) (MinPoint :type "Vector Structure") (MinIndex :type Integer))
  (for (_array_element _array_index) (`self.SplinePointsLocations`)
    (bind _returnvalue (`KismetMathLibrary.Vector_DistanceSquared` _array_element Point))
    (set `local.MinDistanceSquared` (`KismetMathLibrary.FMin` (`local.MinDistanceSquared`) _returnvalue))
    (if (== _returnvalue (`local.MinDistanceSquared`))
      (set `local.MinPoint` _array_element)
      (set `local.MinIndex` _array_index)))
  (return (`local.MinPoint`) (`local.MinIndex`)))

(fn `GetFirstPoint`
  (returns (Location :type "Vector Structure (by ref)"))
  (return (`|GetArrayItem` (`self.SplinePointsLocations`))))

(fn `GetNextPoint`
  (params (Index :type Integer))
  (returns (Location :type "Vector Structure (by ref)") (`Next Index` :type Integer))
  (bind _returnvalue (mod (+ Index 1) (`KismetArrayLibrary.Array_Length` (`self.SplinePointsLocations`))))
  (return (`|GetArrayItem` (`self.SplinePointsLocations`) _returnvalue) _returnvalue))

(fn `UserConstructionScript`
  (for _index (range (`SplineComponent.GetNumberOfSplinePoints` (`self.Spline_route`)))
    (`KismetArrayLibrary.Array_Add` (`self.SplinePointsLocations`) (`SplineComponent.GetLocationAtSplinePoint` (`self.Spline_route`) _index "World"))))